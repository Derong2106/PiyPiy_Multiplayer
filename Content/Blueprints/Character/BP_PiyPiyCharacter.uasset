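; BP_PiyPiyCharacter is the character Blueprint that handles the sniper scope overlay and its zoom feedback.
; ShowSniperScopeWidget lazily creates WBP_SniperScope, adds it to the viewport and keeps the reference for reuse.
; The ShowScope flag plays the widget's single ScopeZoomin animation forward or in reverse, with a matching zoom-in or zoom-out 2D sound.
; All other events and the construction script are empty.
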(event `self.ReceiveBeginPlay`)

(event `self.ShowSniperScopeWidget`
  (params (bShowScope :type Boolean))
  (bind _sniper_scope_widget (`self.Sniper Scope Widget`))
  (bind _sniper_scope_widget_2 (`self.Sniper Scope Widget`))
  (bind _scopezoomin (`/Game/Blueprints/HUD/WBP_SniperScope.ScopeZoomin` _sniper_scope_widget_2))
  (`/Engine/EditorBlueprintResources/StandardMacros.IsValid` (`self.Sniper Scope Widget`)
    (:`Is Valid`
      _)
    (:`Is Not Valid`
      (bind _returnvalue (`|CreateWidget` "/Game/Blueprints/HUD/WBP_SniperScope.WBP_SniperScope_C"))
      (bind _output_get (set `self.Sniper Scope Widget` _returnvalue))
      (`UserWidget.AddToViewport` _output_get 0)))
  (if bShowScope
    (`/Engine/EditorBlueprintResources/StandardMacros.IsValid` _sniper_scope_widget_2
      (:`Is Valid`
        (`UserWidget.PlayAnimation` _sniper_scope_widget _scopezoomin 0.0 1 "Forward" 1.0 false)
        (`GameplayStatics.PlaySound2D` "/Game/Assets/MilitaryWeapSilver/Sound/SniperRifle/Cues/SniperRifle_ZoomIn_Cue.SniperRifle_ZoomIn_Cue" 1.0 1.0 0.0 null null)))
    (else
      (`/Engine/EditorBlueprintResources/StandardMacros.IsValid` _sniper_scope_widget_2
        (:`Is Valid`
          (`UserWidget.PlayAnimation` _sniper_scope_widget _scopezoomin 0.0 1 "Reverse" 1.0 false)
          (`GameplayStatics.PlaySound2D` "/Game/Assets/MilitaryWeapSilver/Sound/SniperRifle/Cues/SniperRifle_ZoomOut_Cue.SniperRifle_ZoomOut_Cue" 1.0 1.0 0.0 null null))))))

(fn `UserConstructionScript`)